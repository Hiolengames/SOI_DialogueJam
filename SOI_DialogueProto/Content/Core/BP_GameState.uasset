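; Game state that coordinates item combining between the two players, Anna and Jacob, whose inventories register with it.
; A server check, once both combo slots are filled, looks up the item pair in the game instance's ComboBase and caches any match.
; Executing a valid combo empties both slots and adds the generated item to Anna's inventory only.
; Multicast events relay combo availability and validation to listeners through dispatchers.
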(event `Server_CheckCombo`
  (bind _itemcomboslot_itemid (break `/Game/Inventory/Structures/S_InventorySlot` (`/Game/Inventory/BPC_InventoryD.itemComboSlot` (`self.AnnaInventoryRef`))))
  (bind _itemcomboslot_itemid_2 (break `/Game/Inventory/Structures/S_InventorySlot` (`/Game/Inventory/BPC_InventoryD.itemComboSlot` (`self.JacobInventoryRef`))))
  (if (and (!= _itemcomboslot_itemid "None") (!= _itemcomboslot_itemid_2 "None"))
    (`self.PairCanCombo`)))

(event `Multicast_UpdateComboState`
  (params (CanCombo :type Boolean) (ComboData :type "/Game/Items/S_Combo Structure"))
  (`self.OnComboStateChanged` CanCombo ComboData_ObjectGenerated_35_3CD93D5B41B853BE5997E983F8EBE17F))

(event `Multicast_ComboValidate`
  (`self.OnComboValidate`))

(fn `ExecuteCombo`
  (bind (_currentcombo_item _currentcombo_item2 _currentcombo_objectgenerated) (break `/Game/Items/S_Combo` (`self.CurrentCombo`)))
  (if (`self.bCanPlayersCombo`)
    (set `self.bCanPlayersCombo` false)
    (setmembers `/Game/Inventory/Structures/S_InventorySlot` :`StructRef` (`/Game/Inventory/BPC_InventoryD.itemComboSlot` (`self.JacobInventoryRef`)) :`ItemID` "None" :`ItemDataAsset` null)
    (setmembers `/Game/Inventory/Structures/S_InventorySlot` :`StructRef` (`/Game/Inventory/BPC_InventoryD.itemComboSlot` (`self.AnnaInventoryRef`)) :`ItemID` "None" :`ItemDataAsset` null)
    (`/Game/Inventory/BPC_InventoryD.AddItem` (`self.AnnaInventoryRef`) (`/Game/Inventory/Library/BFL_Inventory.MakeItemToAdd` (`|ConvertAsset` _currentcombo_objectgenerated)))
    (set `self.CurrentCombo` (struct))
    (`self.Multicast_ComboValidate`)))

(fn `PairCanCombo`
  (locals (Local_CanCombo :type Boolean :default false) (Local_ComboData :type "/Game/Items/S_Combo Structure"))
  (bind (_itemcomboslot_itemid _itemcomboslot_slotindex _itemcomboslot_itemdataasset) (break `/Game/Inventory/Structures/S_InventorySlot` (`/Game/Inventory/BPC_InventoryD.itemComboSlot` (`self.JacobInventoryRef`))))
  (bind (_itemcomboslot_itemid_2 _itemcomboslot_slotindex_2 _itemcomboslot_itemdataasset_2) (break `/Game/Inventory/Structures/S_InventorySlot` (`/Game/Inventory/BPC_InventoryD.itemComboSlot` (`self.AnnaInventoryRef`))))
  (bind _asbp_game_instance (cast `/Game/Core/BP_GameInstance` (`GameplayStatics.GetGameInstance`)))
  (bind (_found _combo) (`/Game/Items/BP_ComboBase.GetCombo` (`/Game/Core/BP_GameInstance.ComboBase` _asbp_game_instance) (`|ConvertAsset` _itemcomboslot_itemdataasset_2) (`|ConvertAsset` _itemcomboslot_itemdataasset)))
  (bind _output_get (set `local.Local_CanCombo` _found))
  (set `self.bCanPlayersCombo` _output_get)
  (bind _output_get_2 (set `local.Local_ComboData` _combo))
  (set `self.CurrentCombo` _output_get_2)
  (`self.Multicast_UpdateComboState` _output_get _output_get_2))

(fn `RegisterPlayerInventory`
  (params (PlayerInventoryRef :type "/Game/Inventory/BPC_InventoryD Object Reference") (IsPlayerAnna :type Boolean))
  (if IsPlayerAnna
    (set `self.AnnaInventoryRef` PlayerInventoryRef)
    (else
      (set `self.JacobInventoryRef` PlayerInventoryRef))))

(fn `UserConstructionScript`)