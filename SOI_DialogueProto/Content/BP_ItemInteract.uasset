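; Interactable pickup item that grants a gameplay tag to the game's state when picked.
; Interact sets the Picked flag once, and its RepNotify calls PickTagObject, which adds the tag to BP_GameInstance's StateTags, prints debug strings and destroys the actor.
; A cosmetic opening-sound event, intended as a multicast to keep sound out of the RepNotify, exists but its call is never run.
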(event `/Game/Dialogue/Core/BPI_Interactable.Interact`
  (params (PlayerThatInteract :type "Actor Object Reference") (`ServerInteract?` :type Boolean))
  ; If add sound to it, use Multicast instead and not in repnotify
  (if (not (`self.Picked?`))
    (set `self.Picked?` true)))

(event `MC_CosmeticOpening`
  (`GameplayStatics.PlaySoundAtLocation` null (0.0 0.0 0.0) (struct) 1.0 1.0 0.0 null null null null))

(event `PickTagObject`
  ; If add sound to it, use Multicast instead and not in repnotify
  (`KismetSystemLibrary.PrintString` "PickTag")
  (bind _asbp_game_instance (cast `/Game/Core/BP_GameInstance` (`GameplayStatics.GetGameInstance`)))
  (`/Game/BP_StateTags.AddGameTag` (`/Game/Core/BP_GameInstance.stateTags` _asbp_game_instance) (`self.GameplayTag`))
  (`KismetSystemLibrary.PrintString` "Added Tag")
  (`self.K2_DestroyActor`))

(fn `OnRep_Picked?`
  (`self.PickTagObject`))

(fn `UserConstructionScript`)