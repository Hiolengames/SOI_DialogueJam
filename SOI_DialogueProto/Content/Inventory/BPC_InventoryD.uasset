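; Inventory component that holds a fixed number of item slots, built on BeginPlay, with Server-prefixed events for setup, adding and transferring items.
; Adding fills the first empty slot, while transfers move an item to a target index or swap if occupied, even across inventories.
; All writes go through SetItem, which restamps the slot's index and owner reference, then fires OnSlotChanged.
; Transfers without a target index only print a message.
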(event `self.ReceiveBeginPlay`
  (`self.Server_SetupSlot` (`self.SlotsAmount`)))

(event `Server_SetupSlot`
  (params (SlotsAmount :type Integer))
  ; Setup Inventory slots on Server
  (bind _output_get (set `self.SlotsAmount` SlotsAmount))
  (for _index (range _output_get)
    (`KismetArrayLibrary.Array_Add` (`self.ItemSlots`) (make `/Game/Inventory/Structures/S_InventorySlot` :`SlotIndex` _index :`InventoryRef` self))))

(event `Server_AddItem`
  (params (ItemToAdd :type "/Game/Inventory/Structures/S_InventorySlot Structure"))
  (`self.AddItem` ItemToAdd))

(event `Server_TransferItem`
  (params (ToInventoryComponent :type "/Game/Inventory/BPC_InventoryD Object Reference") (FromIndex :type Integer) (ToIndex :type Integer))
  (`self.TransferItem` ToInventoryComponent FromIndex ToIndex))

(fn `AddItem`
  (params (ItemToAdd :type "/Game/Inventory/Structures/S_InventorySlot Structure"))
  (returns (Success :type Boolean))
  (bind (_result _slot) (`self.FindEmptySlot`))
  (if _result
    (`self.SetItem` _slot ItemToAdd)
    (else
      (`KismetSystemLibrary.PrintString` "Inventory is full")
      (return false))))

(fn `AddItemToIndex`
  (params (TargetIndex :type Integer) (ItemSlotToAdd :type "/Game/Inventory/Structures/S_InventorySlot Structure"))
  (returns (Success :type Boolean) (Swap :type Boolean))
  (bind (_isvalid _slot) (`self.GetSlotIndex` TargetIndex))
  (if _isvalid
    (if (`/Game/Inventory/Library/BFL_Inventory.IsSlotEmpty` _slot)
      (`self.SetItem` _slot ItemSlotToAdd)
      (return true false)
      (else
        (`self.SwapIndexes` _slot (`local.ItemSlotToAdd`))
        (return true true)))
    (else
      (return false false))))

(fn `FindEmptySlot`
  (returns (Result :type Boolean) (Slot :type "/Game/Inventory/Structures/S_InventorySlot Structure"))
  (for _array_element (`self.ItemSlots`)
    (if (`/Game/Inventory/Library/BFL_Inventory.IsSlotEmpty` _array_element)
      (return true _array_element))))

(fn `GetSlotIndex`
  (params (Index :type Integer))
  (returns (IsValid :type Boolean) (Slot :type "/Game/Inventory/Structures/S_InventorySlot Structure"))
  (if (`KismetArrayLibrary.Array_IsValidIndex` (`self.ItemSlots`) Index)
    (return true (`|GetArrayItem` (`self.ItemSlots`) (`local.Index`)))
    (else
      (return false))))

(fn `RemoveItemFromIndex`
  (params (Index :type Integer))
  (returns (Success :type Boolean))
  (bind (_isvalid _slot) (`self.GetSlotIndex` Index))
  (if _isvalid
    (`self.SetItem` _slot (make `/Game/Inventory/Structures/S_InventorySlot`))
    (return true)
    (else
      (return false))))

(fn `SetItem`
  (params (TargetSlot :type "/Game/Inventory/Structures/S_InventorySlot Structure") (Item :type "/Game/Inventory/Structures/S_InventorySlot Structure"))
  (bind ((`SlotIndex_5_6DECD12143857BAFB66F098E2F75DFB3` _slotindex)) (break `/Game/Inventory/Structures/S_InventorySlot` TargetSlot))
  (`KismetArrayLibrary.Array_Set` (`self.ItemSlots`) _slotindex Item)
  (bind _structout (setmembers `/Game/Inventory/Structures/S_InventorySlot` :`StructRef` (`|GetArrayItem` (`self.ItemSlots`) _slotindex) :`SlotIndex` _slotindex :`InventoryRef` self))
  (`self.OnSlotChanged` _structout))

(fn `SwapIndexes`
  (params (Slot :type "/Game/Inventory/Structures/S_InventorySlot Structure") (SwapWithSlot :type "/Game/Inventory/Structures/S_InventorySlot Structure"))
  (bind _swapwithslot (`local.SwapWithSlot`))
  (`self.SetItem` Slot SwapWithSlot)
  (`self.SetItem` (`.InventoryRef_11_D4B3680E47694BA8063BAF964D529ACC` (break `/Game/Inventory/Structures/S_InventorySlot` _swapwithslot)) _swapwithslot (`local.Slot`)))

(fn `TransferItem`
  (params (ToInventoryComponent :type "/Game/Inventory/BPC_InventoryD Object Reference") (FromIndex :type Integer) (ToIndex :type Integer))
  (returns (Success :type Boolean))
  (bind _toindex (`local.ToIndex`))
  (if (and (== self ToInventoryComponent) (== FromIndex ToIndex))
    (return false)
    (elif (and (`KismetSystemLibrary.IsValid` (`local.ToInventoryComponent`)) (`self.GetSlotIndex` (`local.FromIndex`)) (or (`self.GetSlotIndex` _toindex) (== _toindex -1)))
      (if (== (`local.ToIndex`) -1)
        (`KismetSystemLibrary.PrintString` "Target slot index not specified")
        (else
          (bind (_success _swap) (`self.AddItemToIndex` (`local.ToInventoryComponent`) (`local.ToIndex`) (`.Slot` (`self.GetSlotIndex` (`local.FromIndex`)))))
          (if _success
            (if _swap
              (return true)
              (else
                (bind _success_2 (`self.RemoveItemFromIndex` (`local.FromIndex`)))
                (return _success_2)))
            (else
              (return false)))))
      (else
        (return false)))))