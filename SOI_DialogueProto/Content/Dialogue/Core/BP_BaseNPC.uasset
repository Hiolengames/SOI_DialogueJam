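; Base NPC actor that runs a shared two-player conversation through BPDialogueManager, initialized with a global dialogue asset on BeginPlay.
; Interact starts dialogue on the server when none is active, registering the NPC and two player characters as participants.
; Each player receives client calls to create and fill the dialogue UI with their own choices, then is teleported to a designated spot.
; Dialogue participant functions are default stubs, except the name getter returning DlgName.
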(event `self.ReceiveBeginPlay`
  ; Passing Global Dialogue Asset to Initialize Dialogue Correctly
  (`/Game/Dialogue/Core/BP_DialogueManager.InitializeDialogue` (`self.BP_DialogueManager`) (`self.GlobalDialogue`)))

(event `self.Interact`
  (params (PlayerThatInteract :type "Actor Object Reference") (`ServerInteract?` :type Boolean))
  ; Call StartDialogue function if there is no Active Dialogue and we are on server (authority)
  (`/Engine/EditorBlueprintResources/ActorMacros.Switch Has Authority`
    (:`Authority`
      (if (not (`self.bDialogueActive`))
        (`self.StartDialogue`)))))

(fn `CheckCondition`
  (params (Context :type "DlgContext Object Reference") (ConditionName :type Name))
  (returns (ReturnValue :type Boolean))
  (return false))

(fn `EndDialogue`
  (set `self.bDialogueActive` false))

(fn `GetBoolValue`
  (params (ValueName :type Name))
  (returns (ReturnValue :type Boolean))
  (return false))

(fn `GetFloatValue`
  (params (ValueName :type Name))
  (returns (ReturnValue :type "Float (single-precision)"))
  (return 0.0))

(fn `GetIntValue`
  (params (ValueName :type Name))
  (returns (ReturnValue :type Integer))
  (return 0))

(fn `GetNameValue`
  (params (ValueName :type Name))
  (returns (ReturnValue :type Name))
  (return "None"))

(fn `GetParticipantDisplayName`
  (params (ActiveSpeaker :type Name))
  (returns (ReturnValue :type Text))
  (return ""))

(fn `GetParticipantGender`
  (returns (ReturnValue :type "ETextGender Enum"))
  (return "Masculine"))

(fn `GetParticipantIcon`
  (params (ActiveSpeaker :type Name) (ActiveSpeakerState :type Name))
  (returns (ReturnValue :type "Texture2D Object Reference"))
  (return null))

(fn `GetParticipantName`
  (returns (ReturnValue :type Name))
  (return (`self.DlgName`)))

(fn `ModifyBoolValue`
  (params (ValueName :type Name) (bNewValue :type Boolean))
  (returns (ReturnValue :type Boolean))
  (return false))

(fn `ModifyFloatValue`
  (params (ValueName :type Name) (bDelta :type Boolean) (Value :type "Float (single-precision)"))
  (returns (ReturnValue :type Boolean))
  (return false))

(fn `ModifyIntValue`
  (params (ValueName :type Name) (bDelta :type Boolean) (Value :type Integer))
  (returns (ReturnValue :type Boolean))
  (return false))

(fn `ModifyNameValue`
  (params (ValueName :type Name) (NameValue :type Name))
  (returns (ReturnValue :type Boolean))
  (return false))

(fn `OnDialogueEvent`
  (params (Context :type "DlgContext Object Reference") (EventName :type Name))
  (returns (ReturnValue :type Boolean))
  (return false))

(fn `StartDialogue`
  (bind _playercontroller_ref (`self.PlayerController_Ref`))
  (bind _bp_dialoguemanager (`self.BP_DialogueManager`))
  (bind _bp_dialoguemanager_2 (`self.BP_DialogueManager`))
  (bind _bp_dialoguemanager_3 (`self.BP_DialogueManager`))
  (bind (_returnvalue_location _returnvalue_rotation) (`KismetMathLibrary.BreakTransform` (`SceneComponent.K2_GetComponentToWorld` (`self.Player2TP`))))
  (bind (_returnvalue_location_2 _returnvalue_rotation_2) (`KismetMathLibrary.BreakTransform` (`SceneComponent.K2_GetComponentToWorld` (`self.Player1TP`))))
  ; Get the 3 participants (NPC and both players)
  (bind _outactors (`GameplayStatics.GetAllActorsOfClass` "/Game/ThirdPerson/Blueprints/BP_ThirdPersonCharacter.BP_ThirdPersonCharacter_C"))
  (bind _dialogueended_ (`/Game/Dialogue/Core/BP_DialogueManager.StartCurrentDialogue` (`self.BP_DialogueManager`) (`|MakeArray` self (`|GetArrayItem` _outactors) (`|GetArrayItem` _outactors 1) :!type "Object Object Reference")))
  (if _dialogueended_
    (`self.EndDialogue`)
    (return)
    (else
      (set `self.bDialogueActive` true)
      ; Loop over player controllers to find player 1 & player 2 -> For each Player set up the dialogue UI and set the correct data
      (for _array_element (`GameStateBase.PlayerArray` (`GameplayStatics.GetGameState`))
        (bind _asbp_third_person_player_controller (cast `/Game/ThirdPerson/Blueprints/BP_ThirdPersonPlayerController` (`PlayerState.GetPlayerController` _array_element)))
        (set `self.PlayerController_Ref` _asbp_third_person_player_controller)
        (if (== _asbp_third_person_player_controller (`GameplayStatics.GetPlayerController` 0))
          ; Player 1 - Setup Dialogue Mode & Set Current Dialogue
          (`/Game/ThirdPerson/Blueprints/BP_ThirdPersonPlayerController.Client_CreateDialogueWidget` (`self.PlayerController_Ref`) self)
          (if (`KismetSystemLibrary.IsValid` (`/Game/Dialogue/Core/BP_DialogueManager.Data_ChoiceDialogue_Ref` (`self.BP_DialogueManager`)))
            ; P1 Has Dialogue Choices on StartUp
            (`/Game/ThirdPerson/Blueprints/BP_ThirdPersonPlayerController.Client_UpdateDialogue` (`self.PlayerController_Ref`) (`KismetTextLibrary.Conv_NameToText` (`DlgContext.GetActiveNodeParticipantName` (`/Game/Dialogue/Core/BP_DialogueManager.ActiveContext` _bp_dialoguemanager_2))) (`DlgContext.GetActiveNodeText` (`/Game/Dialogue/Core/BP_DialogueManager.ActiveContext` _bp_dialoguemanager_2)) (`/Game/Dialogue/Core/Data/DialogueChoicesData.DialogueTextP1` (`/Game/Dialogue/Core/BP_DialogueManager.Data_ChoiceDialogue_Ref` _bp_dialoguemanager_2)))
            (else
              ; P1 Doesn't have Dialogue Choices on StartUp
              (`/Game/ThirdPerson/Blueprints/BP_ThirdPersonPlayerController.Client_UpdateDialogue` :`self` (`self.PlayerController_Ref`) :`Speaker` (`KismetTextLibrary.Conv_NameToText` (`DlgContext.GetActiveNodeParticipantName` (`/Game/Dialogue/Core/BP_DialogueManager.ActiveContext` (`self.BP_DialogueManager`)))))))
          ; Teleport Player to P1 Spot
          (`self.K2_TeleportTo` (`Controller.K2_GetPawn` (`self.PlayerController_Ref`)) _returnvalue_location_2 _returnvalue_rotation_2)
          (else
            ; Player2 - Setup Dialogue Mode & Set Current Dialogue
            (`/Game/ThirdPerson/Blueprints/BP_ThirdPersonPlayerController.Client_CreateDialogueWidget` _playercontroller_ref self)
            (if (`KismetSystemLibrary.IsValid` (`/Game/Dialogue/Core/BP_DialogueManager.Data_ChoiceDialogue_Ref` (`self.BP_DialogueManager`)))
              ; P2 Has Dialogue Choices on StartUp
              (`/Game/ThirdPerson/Blueprints/BP_ThirdPersonPlayerController.Client_UpdateDialogue` _playercontroller_ref (`KismetTextLibrary.Conv_NameToText` (`DlgContext.GetActiveNodeParticipantName` (`/Game/Dialogue/Core/BP_DialogueManager.ActiveContext` _bp_dialoguemanager_3))) (`DlgContext.GetActiveNodeText` (`/Game/Dialogue/Core/BP_DialogueManager.ActiveContext` _bp_dialoguemanager_3)) (`/Game/Dialogue/Core/Data/DialogueChoicesData.DialogueTextP2` (`/Game/Dialogue/Core/BP_DialogueManager.Data_ChoiceDialogue_Ref` _bp_dialoguemanager_3)))
              (else
                ; P2 Doesn't have Dialogue Choices on StartUp
                (`/Game/ThirdPerson/Blueprints/BP_ThirdPersonPlayerController.Client_UpdateDialogue` :`self` (`self.PlayerController_Ref`) :`Speaker` (`KismetTextLibrary.Conv_NameToText` (`DlgContext.GetActiveNodeParticipantName` (`/Game/Dialogue/Core/BP_DialogueManager.ActiveContext` _bp_dialoguemanager))) :`Dialogue` (`DlgContext.GetActiveNodeText` (`/Game/Dialogue/Core/BP_DialogueManager.ActiveContext` _bp_dialoguemanager)))))
            ; Teleport Player to P2 Spot
            (`self.K2_TeleportTo` (`Controller.K2_GetPawn` (`self.PlayerController_Ref`)) _returnvalue_location _returnvalue_rotation)))))))

(fn `UserConstructionScript`)