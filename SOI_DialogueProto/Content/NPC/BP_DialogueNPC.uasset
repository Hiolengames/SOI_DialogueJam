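; BP_DialogueNPC is an interactable NPC that runs one shared dialogue for all players in a multiplayer game.
; On Interact, the server starts a dialogue if none is active, using BPDialogueComponent to check item tags and supply the opening data.
; It pushes the dialogue to every player controller through client calls, giving player index 0 the P1 choices and others P2.
; EndDialogueNPC clears the active flag.
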(event `/Game/NPC/BPI_Interactable.Interact`
  (params (PlayerThatInteract :type "Actor Object Reference") (`ServerInteract?` :type Boolean))
  ; Call StartDialogue function if there is no Active Dialogue and we are on server (authority)
  (`/Engine/EditorBlueprintResources/ActorMacros.Switch Has Authority`
    (:`Authority`
      (if (not (`self.bDialogueActive`))
        (`self.StartDialogue`)))))

(fn `EndDialogueNPC`
  (set `self.bDialogueActive` false))

(fn `StartDialogue`
  (bind _bp_dialoguecomponent (`self.BP_DialogueComponent`))
  ; Set dialogue active, verify which dialogue we're at depending on conditions and initialize the dialogue
  (set `self.bDialogueActive` true)
  (`/Game/NPC/BP_DialogueComponent.CheckItemTag` _bp_dialoguecomponent)
  (bind _initdialoguedata (`/Game/NPC/BP_DialogueComponent.InitDialogue` _bp_dialoguecomponent))
  ; For each player, start the dialogue and update it with the data
  (for _array_element (`GameStateBase.PlayerArray` (`GameplayStatics.GetGameState`))
    (bind _asbp_third_person_player_controller (cast `/Game/ThirdPerson/Blueprints/BP_ThirdPersonPlayerController` (`PlayerState.GetPlayerController` _array_element)))
    (`/Game/ThirdPerson/Blueprints/BP_ThirdPersonPlayerController.Client_StartDialogue` _asbp_third_person_player_controller self)
    (if (== _asbp_third_person_player_controller (`GameplayStatics.GetPlayerController` 0))
      (bind (_nodeid _speakername _dialoguetext _nextnodeid _choicesp1 _choicesp2) (break `/Game/Dialogue/S_DialogueNode` _initdialoguedata))
      (`/Game/ThirdPerson/Blueprints/BP_ThirdPersonPlayerController.Client_UpdateDialogueFromNPC` _asbp_third_person_player_controller _speakername _dialoguetext _choicesp1)
      (else
        (`/Game/ThirdPerson/Blueprints/BP_ThirdPersonPlayerController.Client_UpdateDialogueFromNPC` _asbp_third_person_player_controller _speakername _dialoguetext _choicesp2)))))

(fn `UserConstructionScript`)