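; BP_LoadAndUnload is a trigger actor that streams levels in and out as the third-person character overlaps its two boxes.
; EntryBox asynchronously loads LevelToLoad and makes it visible.
; ExitBox asynchronously unloads LevelToUnload, but only once DoorActive is set after a short delay from BeginPlay, so overlaps at startup do not unload it.
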(event `self.ReceiveBeginPlay`
  (`KismetSystemLibrary.Delay` 0.5)
  (set `self.bDoorActive` true))

(event `self.Entry Box.OnComponentBeginOverlap`
  (params (OverlappedComponent :type "PrimitiveComponent Object Reference") (OtherActor :type "Actor Object Reference") (OtherComp :type "PrimitiveComponent Object Reference") (OtherBodyIndex :type Integer) (bFromSweep :type Boolean) (SweepResult :type "HitResult Structure (by ref)"))
  (cast `/Game/ThirdPerson/Blueprints/BP_ThirdPersonCharacter` OtherActor)
  (`GameplayStatics.LoadStreamLevelBySoftObjectPtr` (`self.LevelToLoad`) true))

(event `self.Exit Box.OnComponentBeginOverlap`
  (params (OverlappedComponent :type "PrimitiveComponent Object Reference") (OtherActor :type "Actor Object Reference") (OtherComp :type "PrimitiveComponent Object Reference") (OtherBodyIndex :type Integer) (bFromSweep :type Boolean) (SweepResult :type "HitResult Structure (by ref)"))
  (cast `/Game/ThirdPerson/Blueprints/BP_ThirdPersonCharacter` OtherActor)
  (if (`self.bDoorActive`)
    (`GameplayStatics.UnloadStreamLevelBySoftObjectPtr` (`self.LevelToUnload`))))

(fn `UserConstructionScript`)