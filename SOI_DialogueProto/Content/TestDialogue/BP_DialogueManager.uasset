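; Dialogue manager component for an NPC that runs branching conversations shared by two players.
; A global dialogue graph selects the current conversation asset, and that conversation's final choice ID advances the global graph to the next one.
; Both players' picks are combined into one positive, negative, orange or violet outcome, remapped for three-option nodes.
; Player controllers receive speaker, text and per-player options through client update calls, plus an end-of-dialogue reset.
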(fn `AdvanceDialogue`
  (bind _returnvalue (`DlgContext.GetActiveNodeData` (`self.ActiveContext`)))
  ; Advances the Dialogue from Confirmed Choices, based on both players's answers
  (if (`self.bDialogueActive`)
    (set `self.Data_ChoiceDialogue_Ref` null)
    (`/Engine/EditorBlueprintResources/StandardMacros.IsValid` _returnvalue
      (:`Is Valid`
        (bind _asdialogue_choices_data (cast `/Game/TestDialogue/DialogueChoicesData` _returnvalue))
        (set `self.Data_ChoiceDialogue_Ref` _asdialogue_choices_data))
      (:`Is Not Valid`
        _))
    (for _array_element (`GameStateBase.PlayerArray` (`GameplayStatics.GetGameState`))
      (bind _asbp_third_person_player_controller (cast `/Game/ThirdPerson/Blueprints/BP_ThirdPersonPlayerController` (`PlayerState.GetPlayerController` _array_element)))
      (set `self.PlayerController_Ref` _asbp_third_person_player_controller)
      (if (== _asbp_third_person_player_controller (`GameplayStatics.GetPlayerController` 0))
        ; Player 1 - Update Current Dialogue if choices are available
        (if (`KismetSystemLibrary.IsValid` (`self.Data_ChoiceDialogue_Ref`))
          ; Player 1 has dialogue choices -> Update the Dialogue on Client
          (`/Game/ThirdPerson/Blueprints/BP_ThirdPersonPlayerController.Client_UpdateDialogue` (`self.PlayerController_Ref`) (`KismetTextLibrary.Conv_NameToText` (`DlgContext.GetActiveNodeParticipantName` (`self.ActiveContext`))) (`DlgContext.GetActiveNodeText` (`self.ActiveContext`)) (`/Game/TestDialogue/DialogueChoicesData.DialogueTextP1` (`self.Data_ChoiceDialogue_Ref`)))
          (else
            ; Player 1 has NO dialogue choices -> Update the Dialogue on Client
            (`/Game/ThirdPerson/Blueprints/BP_ThirdPersonPlayerController.Client_UpdateDialogue` :`self` (`self.PlayerController_Ref`) :`Speaker` (`KismetTextLibrary.Conv_NameToText` (`DlgContext.GetActiveNodeParticipantName` (`self.ActiveContext`))) :`Dialogue` (`DlgContext.GetActiveNodeText` (`self.ActiveContext`)))))
        (else
          ; Player 2 - Update Dialogue after choice
          (if (`KismetSystemLibrary.IsValid` (`self.Data_ChoiceDialogue_Ref`))
            ; Player 2 has dialogue choices -> Update the Dialogue on Client
            (`/Game/ThirdPerson/Blueprints/BP_ThirdPersonPlayerController.Client_UpdateDialogue` (`self.PlayerController_Ref`) (`KismetTextLibrary.Conv_NameToText` (`DlgContext.GetActiveNodeParticipantName` (`self.ActiveContext`))) (`DlgContext.GetActiveNodeText` (`self.ActiveContext`)) (`/Game/TestDialogue/DialogueChoicesData.DialogueTextP2` (`self.Data_ChoiceDialogue_Ref`)))
            (else
              ; Player 2 has NO dialogue choices -> Update the Dialogue on Client
              (`/Game/ThirdPerson/Blueprints/BP_ThirdPersonPlayerController.Client_UpdateDialogue` :`self` (`self.PlayerController_Ref`) :`Speaker` (`KismetTextLibrary.Conv_NameToText` (`DlgContext.GetActiveNodeParticipantName` (`self.ActiveContext`))) :`Dialogue` (`DlgContext.GetActiveNodeText` (`self.ActiveContext`))))))))
    (else
      (`self.EndDialogueOnClient`)
      (return))))

(fn `EndCurrentDialogue`
  (params (FinalChoiceID :type Integer))
  ; Reset Current Dialogue related variables (since it's over)
  (set `self.CurrentDialogue` null)
  (set `self.bDialogueActive` false)
  (if (`DlgContext.HasDialogueEnded` (`self.GlobalActiveContext`))
    (`self.EndDialogueOnClient`)
    (elif (< FinalChoiceID (`KismetArrayLibrary.Array_Length` (`DlgContext.GetOptionsArray` (`self.GlobalActiveContext`))))
      (`DlgContext.ChooseOption` (`self.GlobalActiveContext`) FinalChoiceID)
      (`self.SetNextDialogueAsset`)
      (`self.EndDialogueOnClient`)
      (else
        (`self.EndDialogueOnClient`)))))

(fn `EndDialogueOnClient`
  ; End Dialogue On Client -> Reset the Choice Values and Call Client to reset the dialogue UI
  (set `self.ActiveContext` null)
  (set `self.bDialogueActive` false)
  (for _array_element (`GameStateBase.PlayerArray` (`GameplayStatics.GetGameState`))
    (bind _asbp_third_person_player_controller (cast `/Game/ThirdPerson/Blueprints/BP_ThirdPersonPlayerController` (`PlayerState.GetPlayerController` _array_element)))
    (`self.ResetDialogueChoiceValues`)
    (`/Game/ThirdPerson/Blueprints/BP_ThirdPersonPlayerController.Client_OnDialogueEnd` _asbp_third_person_player_controller)))

(fn `FindPlayerChoiceFinalResult`
  (returns (ChoiceID :type Integer))
  ; Return the correct ChoiceID value depending on choices of player 1 and 2 (Positif, Negatif, Orange, Violet) ID Value = 0 =positif / 1 = orange / 2 = Violet / 3 = Rouge
  (if (>= (`self.TotalPointsChoice`) 2)
    (`KismetSystemLibrary.PrintString` "Choix positif")
    (return 0)
    (elif (<= (`self.TotalPointsChoice`) -2)
      (`KismetSystemLibrary.PrintString` "Choix negatif")
      (return 3)
      (elif (== (`self.ChoiceID_P1`) (`self.ChoiceID_P2`))
        (`KismetSystemLibrary.PrintString` "Orange")
        (return 1)
        (else
          (`KismetSystemLibrary.PrintString` "Violet")
          (return 2))))))

(fn `InitializeDialogue`
  (params (GlobalDialogueAsset :type "DlgDialogue Object Reference"))
  ; Initializing Global Dialogue Asset as the Current Dialogue
  (bind _returnvalue (`DlgManager.StartDialogue` GlobalDialogueAsset (`|MakeArray` (`self.GetOwner`) :!type "Object Object Reference")))
  (bind _output_get (set `self.GlobalActiveContext` _returnvalue))
  (bind _asdialogue_data_npc (cast `/Game/TestDialogue/DialogueDataNPC` (`DlgContext.GetActiveNodeData` _output_get)))
  (bind _output_get_2 (set `self.Data_NPC_Dialogue_Ref` _asdialogue_data_npc))
  (set `self.CurrentDialogue` (`/Game/TestDialogue/DialogueDataNPC.DialogueNPC` _output_get_2))
  (set `self.FinalChoiceID` -1))

(fn `OnChoiceClicked`
  (params (ChoiceValue :type Integer) (`PlayerController Ref` :type "/Game/ThirdPerson/Blueprints/BP_ThirdPersonPlayerController Object Reference"))
  (bind _activecontext (`self.ActiveContext`))
  (bind _activecontext_2 (`self.ActiveContext`))
  ; Update "ChoiceID_P1" or "ChoiceID_P2" int variable depending on which  player is calling the function
  (if (`self.bDialogueActive`)
    (if (== `PlayerController Ref` (`GameplayStatics.GetPlayerController` 0))
      (set `self.ChoiceID_P1` ChoiceValue)
      (else
        (set `self.ChoiceID_P2` ChoiceValue)))
    ; If both players have selected a choice (ChoiceIDP1/2 != -1) then TotalPointChoice is calculated
    (if (and (!= (`self.ChoiceID_P1`) -1) (!= (`self.ChoiceID_P2`) -1))
      (set `self.TotalPointsChoice` (+ (`self.ChoiceID_P1`) (`self.ChoiceID_P2`)))
      (bind _choiceid (`self.FindPlayerChoiceFinalResult`)) ; Find the common ground based on player responses
      (set `self.FinalChoiceID` _choiceid)
      ; If 3 responses available -> follow exec pin 3
      ; If 4 responses available -> follow exec pin 4
      (switch `int` (`KismetArrayLibrary.Array_Length` (`DlgContext.GetOptionsArray` (`self.ActiveContext`)))
        (:`3`
          ; Select the remapped Choice, and advance to next dialogue
          (`DlgContext.ChooseOption` _activecontext (select `int` _choiceid :`0` 0 :`1` 1 :`2` 1 :`3` 2))
          (if (not (`DlgContext.HasDialogueEnded` _activecontext))
            (`self.ResetDialogueChoiceValues`)
            (`self.AdvanceDialogue`)))
        (:`4`
          ; Select the FinalChoice if it is in bounds, and advance to next dialogue
          (`DlgContext.ChooseOption` _activecontext_2 _choiceid)
          (if (not (`DlgContext.HasDialogueEnded` _activecontext_2))
            (`self.ResetDialogueChoiceValues`)
            (`self.AdvanceDialogue`)))))))

(fn `OnNextClicked`
  (params (PlayerController_Ref :type "/Game/ThirdPerson/Blueprints/BP_ThirdPersonPlayerController Object Reference"))
  ; Check If Node Has Multiple Choices
  (if (> (`DlgContext.GetOptionsNum` (`self.ActiveContext`)) 1)
    (`KismetSystemLibrary.PrintString` "Dialogue Has Choices")
    (return)
    (elif (== PlayerController_Ref (`GameplayStatics.GetPlayerController` 0))
      ; Player 1 - Advance Dialogue
      (`DlgContext.ChooseOption` (`self.ActiveContext`) 0)
      (if (`DlgContext.HasDialogueEnded` (`self.ActiveContext`))
        (`self.EndCurrentDialogue` (`self.FinalChoiceID`))
        (return)
        (else
          (`self.ResetDialogueChoiceValues`)
          (`self.AdvanceDialogue`)))
      (else
        ; Player 2 - Advance Dialogue
        (`DlgContext.ChooseOption` (`self.ActiveContext`) 0)
        (if (`DlgContext.HasDialogueEnded` (`self.ActiveContext`))
          (`self.EndCurrentDialogue` (`self.FinalChoiceID`))
          (return)
          (else
            (`self.ResetDialogueChoiceValues`)
            (`self.AdvanceDialogue`)))))))

(fn `ResetDialogueChoiceValues`
  ; Reset Dialogue Values if there was a choice
  (set `self.ChoiceID_P1` -1)
  (set `self.ChoiceID_P2` -1)
  (set `self.TotalPointsChoice` 0))

(fn `SetNextDialogueAsset`
  (bind _asdialogue_data_npc (cast `/Game/TestDialogue/DialogueDataNPC` (`DlgContext.GetActiveNodeData` (`self.GlobalActiveContext`))))
  (bind _output_get (set `self.CurrentDialogue` (`/Game/TestDialogue/DialogueDataNPC.DialogueNPC` _asdialogue_data_npc)))
  (`KismetSystemLibrary.PrintString` (`KismetSystemLibrary.GetDisplayName` _output_get))
  (set `self.FinalChoiceID` -1))

(fn `StartCurrentDialogue`
  (params (Participants :type "Array of Object Object Reference (by ref)"))
  (returns (`DialogueEnded?` :type Boolean))
  (`/Engine/EditorBlueprintResources/StandardMacros.IsValid` (`self.CurrentDialogue`)
    (:`Is Valid`
      ; Start the Dialogue Graph
      (bind _returnvalue (`DlgManager.StartDialogue` (`self.CurrentDialogue`) Participants))
      ; Set Active Context (Current Dialogue) and set the Dialogue Choice Data (responses that are possible in this given dialogue)
      (`/Engine/EditorBlueprintResources/StandardMacros.IsValid` _returnvalue
        (:`Is Valid`
          (bind _output_get (set `self.ActiveContext` _returnvalue))
          (bind _returnvalue_2 (`DlgContext.GetActiveNodeData` _output_get))
          (`/Engine/EditorBlueprintResources/StandardMacros.IsValid` _returnvalue_2
            (:`Is Valid`
              (bind _asdialogue_choices_data (cast `/Game/TestDialogue/DialogueChoicesData` _returnvalue_2))
              (set `self.Data_ChoiceDialogue_Ref` _asdialogue_choices_data)
              (set `self.bDialogueActive` true))
            (:`Is Not Valid`
              _))
          (return false) ; Goes back to BP_NPC StartDialogue()
        )))
    (:`Is Not Valid`
      ; Safety check, if no current dialogue available end dialogue
      (`KismetSystemLibrary.PrintString` "No current dialogue")
      (`self.EndDialogueOnClient`)
      (set `self.bDialogueActive` false)
      (return true))))