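; NPC actor that runs a shared two-player branching conversation as a dialogue participant.
; On server interact it starts the current dialogue and sends text and per-player options to each controller's client widget.
; Both players' choices are combined into one of four outcomes, remapped for three-option nodes.
; A global dialogue acts as story progression: when a conversation ends, the last outcome advances it to select the NPC's next dialogue asset.
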(event `self.ReceiveBeginPlay`
  (bind _returnvalue (`DlgManager.StartDialogue` (`self.GlobalDialogue`) (`|MakeArray` self :!type "Object Object Reference")))
  (bind _output_get (set `self.GlobalActiveContext` _returnvalue))
  (bind _asdialogue_data_npc (cast `/Game/TestDialogue/DialogueDataNPC` (`DlgContext.GetActiveNodeData` _output_get)))
  (bind _output_get_2 (set `self.DialogueDataNPC_Ref` _asdialogue_data_npc))
  (set `self.CurrentDialogue` (`/Game/TestDialogue/DialogueDataNPC.DialogueNPC` _output_get_2))
  (set `self.FinalChoiceID` -1))

(event `self.Interact`
  (params (PlayerThatInteract :type "Actor Object Reference") (`ServerInteract?` :type Boolean))
  (bind _playercontroller_ref (`self.PlayerController_Ref`))
  ; OnInteract Button Pressed -> Start Dialogue with 3 participants
  (`/Engine/EditorBlueprintResources/ActorMacros.Switch Has Authority`
    (:`Authority`
      (if (not (`self.bDialogueActive`))
        (bind _outactors (`GameplayStatics.GetAllActorsOfClass` "/Game/ThirdPerson/Blueprints/BP_ThirdPersonCharacter.BP_ThirdPersonCharacter_C"))
        (bind _returnvalue (`DlgManager.StartDialogue` (`self.CurrentDialogue`) (`|MakeArray` self (`|GetArrayItem` _outactors) (`|GetArrayItem` _outactors 1) :!type "Object Object Reference")))
        (set `self.bDialogueActive` true)
        ; Set Active Context (Current Dialogue) and set the Dialogue Choice Data (responses that are possible in this given dialogue)
        (`/Engine/EditorBlueprintResources/StandardMacros.IsValid` _returnvalue
          (:`Is Valid`
            (bind _output_get (set `self.ActiveContext` _returnvalue))
            (bind _returnvalue_2 (`DlgContext.GetActiveNodeData` _output_get))
            (`/Engine/EditorBlueprintResources/StandardMacros.IsValid` _returnvalue_2
              (:`Is Valid`
                (bind _asdialogue_choices_data (cast `/Game/TestDialogue/DialogueChoicesData` _returnvalue_2))
                (set `self.DialogueChoiceData_Ref` _asdialogue_choices_data))
              (:`Is Not Valid`
                _))
            ; Loop over player controllers to find player 1 & player 2
            (for _array_element (`GameStateBase.PlayerArray` (`GameplayStatics.GetGameState`))
              (bind _asbp_third_person_player_controller (cast `/Game/ThirdPerson/Blueprints/BP_ThirdPersonPlayerController` (`PlayerState.GetPlayerController` _array_element)))
              (set `self.PlayerController_Ref` _asbp_third_person_player_controller)
              (if (== _asbp_third_person_player_controller (`GameplayStatics.GetPlayerController` 0))
                ; Player 1 - Setup Dialogue Mode & Set Current Dialogue
                (`/Game/ThirdPerson/Blueprints/BP_ThirdPersonPlayerController.Client_CreateDialogueWidget` (`self.PlayerController_Ref`) self)
                (if (`KismetSystemLibrary.IsValid` (`self.DialogueChoiceData_Ref`))
                  ; P1 Has Dialogue Choices on StartUp
                  (`/Game/ThirdPerson/Blueprints/BP_ThirdPersonPlayerController.Client_UpdateDialogue` (`self.PlayerController_Ref`) (`KismetTextLibrary.Conv_NameToText` (`DlgContext.GetActiveNodeParticipantName` (`self.ActiveContext`))) (`DlgContext.GetActiveNodeText` (`self.ActiveContext`)) (`/Game/TestDialogue/DialogueChoicesData.DialogueTextP1` (`self.DialogueChoiceData_Ref`)))
                  (else
                    ; P1 Doesn't have Dialogue Choices on StartUp
                    (`/Game/ThirdPerson/Blueprints/BP_ThirdPersonPlayerController.Client_UpdateDialogue` :`self` (`self.PlayerController_Ref`) :`Speaker` (`KismetTextLibrary.Conv_NameToText` (`DlgContext.GetActiveNodeParticipantName` (`self.ActiveContext`))) :`Dialogue` (`DlgContext.GetActiveNodeText` (`self.ActiveContext`)))))
                (else
                  ; Player2 - Setup Dialogue Mode & Set Current Dialogue
                  (`/Game/ThirdPerson/Blueprints/BP_ThirdPersonPlayerController.Client_CreateDialogueWidget` _playercontroller_ref self)
                  (if (`KismetSystemLibrary.IsValid` (`self.DialogueChoiceData_Ref`))
                    ; P2 Has Dialogue Choices on StartUp
                    (`/Game/ThirdPerson/Blueprints/BP_ThirdPersonPlayerController.Client_UpdateDialogue` _playercontroller_ref (`KismetTextLibrary.Conv_NameToText` (`DlgContext.GetActiveNodeParticipantName` (`self.ActiveContext`))) (`DlgContext.GetActiveNodeText` (`self.ActiveContext`)) (`/Game/TestDialogue/DialogueChoicesData.DialogueTextP2` (`self.DialogueChoiceData_Ref`)))
                    (else
                      ; P2 Doesn't have Dialogue Choices on StartUp
                      (`/Game/ThirdPerson/Blueprints/BP_ThirdPersonPlayerController.Client_UpdateDialogue` :`self` (`self.PlayerController_Ref`) :`Speaker` (`KismetTextLibrary.Conv_NameToText` (`DlgContext.GetActiveNodeParticipantName` (`self.ActiveContext`))) :`Dialogue` (`DlgContext.GetActiveNodeText` (`self.ActiveContext`)))))))))
          (:`Is Not Valid`
            (`KismetSystemLibrary.PrintString` "Active context is not valid")))))))

(event `AdvanceDialogueFromChoices`
  (bind _returnvalue (`DlgContext.GetActiveNodeData` (`self.ActiveContext`)))
  ; Advances the Dialogue from Confirmed Choices, based on both players's answers
  (set `self.DialogueChoiceData_Ref` null)
  (`/Engine/EditorBlueprintResources/StandardMacros.IsValid` _returnvalue
    (:`Is Valid`
      (bind _asdialogue_choices_data (cast `/Game/TestDialogue/DialogueChoicesData` _returnvalue))
      (set `self.DialogueChoiceData_Ref` _asdialogue_choices_data))
    (:`Is Not Valid`
      _))
  (for _array_element (`GameStateBase.PlayerArray` (`GameplayStatics.GetGameState`))
    (bind _asbp_third_person_player_controller (cast `/Game/ThirdPerson/Blueprints/BP_ThirdPersonPlayerController` (`PlayerState.GetPlayerController` _array_element)))
    (set `self.PlayerController_Ref` _asbp_third_person_player_controller)
    (if (== _asbp_third_person_player_controller (`GameplayStatics.GetPlayerController` 0))
      ; Player 1 - Update Current Dialogue after choice
      (if (`KismetSystemLibrary.IsValid` (`self.DialogueChoiceData_Ref`))
        (`/Game/ThirdPerson/Blueprints/BP_ThirdPersonPlayerController.Client_UpdateDialogue` (`self.PlayerController_Ref`) (`KismetTextLibrary.Conv_NameToText` (`DlgContext.GetActiveNodeParticipantName` (`self.ActiveContext`))) (`DlgContext.GetActiveNodeText` (`self.ActiveContext`)) (`/Game/TestDialogue/DialogueChoicesData.DialogueTextP1` (`self.DialogueChoiceData_Ref`)))
        (else
          (`/Game/ThirdPerson/Blueprints/BP_ThirdPersonPlayerController.Client_UpdateDialogue` :`self` (`self.PlayerController_Ref`) :`Speaker` (`KismetTextLibrary.Conv_NameToText` (`DlgContext.GetActiveNodeParticipantName` (`self.ActiveContext`))) :`Dialogue` (`DlgContext.GetActiveNodeText` (`self.ActiveContext`)))))
      (else
        ; Player 2 - Update Dialogue after choice
        (if (`KismetSystemLibrary.IsValid` (`self.DialogueChoiceData_Ref`))
          (`/Game/ThirdPerson/Blueprints/BP_ThirdPersonPlayerController.Client_UpdateDialogue` (`self.PlayerController_Ref`) (`KismetTextLibrary.Conv_NameToText` (`DlgContext.GetActiveNodeParticipantName` (`self.ActiveContext`))) (`DlgContext.GetActiveNodeText` (`self.ActiveContext`)) (`/Game/TestDialogue/DialogueChoicesData.DialogueTextP2` (`self.DialogueChoiceData_Ref`)))
          (else
            (`/Game/ThirdPerson/Blueprints/BP_ThirdPersonPlayerController.Client_UpdateDialogue` :`self` (`self.PlayerController_Ref`) :`Speaker` (`KismetTextLibrary.Conv_NameToText` (`DlgContext.GetActiveNodeParticipantName` (`self.ActiveContext`))) :`Dialogue` (`DlgContext.GetActiveNodeText` (`self.ActiveContext`)))))))))

(fn `CheckCondition`
  (params (Context :type "DlgContext Object Reference") (ConditionName :type Name))
  (returns (ReturnValue :type Boolean))
  (return false))

(fn `ChoiceAdvanceDialogue`
  (params (PlayerController :type "/Game/ThirdPerson/Blueprints/BP_ThirdPersonPlayerController Object Reference") (ChoiceValue :type Integer))
  (bind _activecontext (`self.ActiveContext`))
  (bind _activecontext_2 (`self.ActiveContext`))
  ; Update "ChoiceID_P1" or "ChoiceID_P2" int variable depending on which  player is calling the function
  (if (== PlayerController (`GameplayStatics.GetPlayerController` 0))
    (set `self.ChoiceID_P1` ChoiceValue)
    (else
      (set `self.ChoiceID_P2` ChoiceValue)))
  ; If both players have selected a choice (ChoiceIDP1/2 != -1) then TotalPointChoice is calculated
  (if (and (!= (`self.ChoiceID_P1`) -1) (!= (`self.ChoiceID_P2`) -1))
    (set `self.TotalPointsChoice` (+ (`self.ChoiceID_P1`) (`self.ChoiceID_P2`)))
    (bind _choiceid (`self.FindPlayerChoiceFinalResult`)) ; Find the common ground based on player responses
    (set `self.FinalChoiceID` _choiceid)
    ; Choice Remapping based on the Amount of Options we have
    ;;[0.04167 0.04167 0.04167 0.5] Determine how many response nodes exist in the current context. Changes execution to the correct logic based on tree density
    (switch `int` (`KismetArrayLibrary.Array_Length` (`DlgContext.GetOptionsArray` (`self.ActiveContext`))) ; Case 3 -> Handles 3-node responses\nCase 4 -> Handles 4-node responses
      (:`3`
        ;;[0.04167 0.04167 0.04167 0.5] 3 responses exist in the dialogue structure, so the remapped FinalChoiceID is used
        ;; (Select the Choice based on the remapped index, and advance to next dialogue)
        (`DlgContext.ChooseOption` _activecontext (select `int` _choiceid :`0` 0 :`1` 1 :`2` 1 :`3` 2))
        (if (not (`DlgContext.HasDialogueEnded` _activecontext))
          (`self.ResetChoiceValues`)
          (`self.AdvanceDialogueFromChoices`)))
      (:`4`
        ;;[0.04167 0.04167 0.04167 0.5] All four responses exist in the dialogue structure, so the calculated FinalChoiceID can be used directly, no remap needed
        ;; (Select the FinalChoice based on calculated index, and advance to next dialogue)
        (`DlgContext.ChooseOption` _activecontext_2 _choiceid)
        (if (not (`DlgContext.HasDialogueEnded` _activecontext_2))
          (`self.ResetChoiceValues`)
          (`self.AdvanceDialogueFromChoices`))))))

(fn `EndCurrentDialogue`
  (params (FinalChoiceID :type Integer))
  (set `self.CurrentDialogue` null)
  (set `self.bDialogueActive` false)
  (if (`DlgContext.HasDialogueEnded` (`self.GlobalActiveContext`))
    (`self.EndDialogueOnClient`)
    (elif (and (>= FinalChoiceID 0) (< FinalChoiceID (`KismetArrayLibrary.Array_Length` (`DlgContext.GetOptionsArray` (`self.GlobalActiveContext`)))))
      (`DlgContext.ChooseOption` (`self.GlobalActiveContext`) FinalChoiceID)
      (`self.SetNextDialogueAsset`)
      (`self.EndDialogueOnClient`)
      (else
        (`self.EndDialogueOnClient`)))))

(fn `EndDialogueOnClient`
  (for _array_element (`GameStateBase.PlayerArray` (`GameplayStatics.GetGameState`))
    (bind _asbp_third_person_player_controller (cast `/Game/ThirdPerson/Blueprints/BP_ThirdPersonPlayerController` (`PlayerState.GetPlayerController` _array_element)))
    (`self.ResetChoiceValues`)
    (`/Game/ThirdPerson/Blueprints/BP_ThirdPersonPlayerController.Client_OnDialogueEnd` _asbp_third_person_player_controller)))

(fn `FindPlayerChoiceFinalResult`
  (returns (ChoiceID :type Integer))
  ; Return the correct ChoiceID value depending on choices of player 1 and 2 (Positif, Negatif, Orange, Violet) ID Value = 0 =positif / 1 = orange / 2 = Violet / 3 = Rouge
  (if (>= (`self.TotalPointsChoice`) 2)
    (`KismetSystemLibrary.PrintString` "Choix positif")
    (return 0)
    (elif (<= (`self.TotalPointsChoice`) -2)
      (`KismetSystemLibrary.PrintString` "Choix negatif")
      (return 3)
      (elif (== (`self.ChoiceID_P1`) (`self.ChoiceID_P2`))
        (`KismetSystemLibrary.PrintString` "Orange")
        (return 1)
        (else
          (`KismetSystemLibrary.PrintString` "Violet")
          (return 2))))))

(fn `GetBoolValue`
  (params (ValueName :type Name))
  (returns (ReturnValue :type Boolean))
  (return false))

(fn `GetFloatValue`
  (params (ValueName :type Name))
  (returns (ReturnValue :type "Float (single-precision)"))
  (return 0.0))

(fn `GetIntValue`
  (params (ValueName :type Name))
  (returns (ReturnValue :type Integer))
  (return 0))

(fn `GetNameValue`
  (params (ValueName :type Name))
  (returns (ReturnValue :type Name))
  (return "None"))

(fn `GetParticipantDisplayName`
  (params (ActiveSpeaker :type Name))
  (returns (ReturnValue :type Text))
  (return ""))

(fn `GetParticipantGender`
  (returns (ReturnValue :type "ETextGender Enum"))
  (return "Masculine"))

(fn `GetParticipantIcon`
  (params (ActiveSpeaker :type Name) (ActiveSpeakerState :type Name))
  (returns (ReturnValue :type "Texture2D Object Reference"))
  (return null))

(fn `GetParticipantName`
  (returns (ReturnValue :type Name))
  (return (`self.DlgName`)))

(fn `ModifyBoolValue`
  (params (ValueName :type Name) (bNewValue :type Boolean))
  (returns (ReturnValue :type Boolean))
  (return false))

(fn `ModifyFloatValue`
  (params (ValueName :type Name) (bDelta :type Boolean) (Value :type "Float (single-precision)"))
  (returns (ReturnValue :type Boolean))
  (return false))

(fn `ModifyIntValue`
  (params (ValueName :type Name) (bDelta :type Boolean) (Value :type Integer))
  (returns (ReturnValue :type Boolean))
  (return false))

(fn `ModifyNameValue`
  (params (ValueName :type Name) (NameValue :type Name))
  (returns (ReturnValue :type Boolean))
  (return false))

(fn `NextDialogueClicked`
  (params (PlayerController :type "/Game/ThirdPerson/Blueprints/BP_ThirdPersonPlayerController Object Reference"))
  ; Check If Node Has Multiple Choices
  (if (> (`DlgContext.GetOptionsNum` (`self.ActiveContext`)) 1)
    (`KismetSystemLibrary.PrintString` "Dialogue Has Choices")
    (return)
    (elif (== PlayerController (`GameplayStatics.GetPlayerController` 0))
      ; Player 1 - Advance Dialogue
      (`DlgContext.ChooseOption` (`self.ActiveContext`) 0)
      (if (`DlgContext.HasDialogueEnded` (`self.ActiveContext`))
        (`self.EndCurrentDialogue` (`self.FinalChoiceID`))
        (return)
        (else
          (`self.ResetChoiceValues`)
          (`self.AdvanceDialogueFromChoices`)))
      (else
        ; Player 2 - Advance Dialogue
        (`DlgContext.ChooseOption` (`self.ActiveContext`) 0)
        (if (`DlgContext.HasDialogueEnded` (`self.ActiveContext`))
          (`self.EndCurrentDialogue` (`self.FinalChoiceID`))
          (return)
          (else
            (`self.ResetChoiceValues`)
            (`self.AdvanceDialogueFromChoices`)))))))

(fn `OnDialogueEvent`
  (params (Context :type "DlgContext Object Reference") (EventName :type Name))
  (returns (ReturnValue :type Boolean))
  (return false))

(fn `ResetChoiceValues`
  ; Reset Dialogue Values if there was a choice
  (set `self.ChoiceID_P1` -1)
  (set `self.ChoiceID_P2` -1)
  (set `self.TotalPointsChoice` 0))

(fn `SetNextDialogueAsset`
  (bind _asdialogue_data_npc (cast `/Game/TestDialogue/DialogueDataNPC` (`DlgContext.GetActiveNodeData` (`self.GlobalActiveContext`))))
  (bind _output_get (set `self.CurrentDialogue` (`/Game/TestDialogue/DialogueDataNPC.DialogueNPC` _asdialogue_data_npc)))
  (`KismetSystemLibrary.PrintString` (`KismetSystemLibrary.GetDisplayName` _output_get))
  (set `self.FinalChoiceID` -1))

(fn `UserConstructionScript`)