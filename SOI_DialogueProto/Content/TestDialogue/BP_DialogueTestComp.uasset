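; NPC dialogue component that runs branching conversations for two players and pushes text and per-player choices to their controllers.
; A dialogue table selects the current node table, whose rows drive each line.
; Both players' choices combine into one of four outcomes, selecting the next node and the NPC's following dialogue.
; GameInstance state tags can override the current dialogue, and authority binds GameMode save/load dispatchers to persist its ID per NPC.
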(event `self.ReceiveBeginPlay`
  ; Set the first Dialogue of the NPC when created
  (bind _returnvalue (`|GetDataTableRow` (`self.DialogueTable`) (`self.CurrentDialogueID`))
    (:`then`
      (bind _output_get (set `self.CurrentDialogueData` _returnvalue))
      (set `self.currentDialogueTable` (break `/Game/Dialogue/S_DialogueStruct` _output_get))
      ; OnSave and OnLoad event dispatchers from GameMode called so it can save the data of where the players are in the dialogue hierarchy
      (`/Engine/EditorBlueprintResources/ActorComponentMacros.Switch Has Authority`
        (:`Authority`
          (bind _asbp_third_person_game_mode (cast `/Game/ThirdPerson/Blueprints/BP_ThirdPersonGameMode` (`GameplayStatics.GetGameMode`)))
          (add `/Game/ThirdPerson/Blueprints/BP_ThirdPersonGameMode.OnSave` _asbp_third_person_game_mode (delegate `OnSave_Event`))
          (add `/Game/ThirdPerson/Blueprints/BP_ThirdPersonGameMode.OnLoad` _asbp_third_person_game_mode (delegate `OnLoad_Event`)))))))

(event `OnSave_Event`
  (params (SaveGame :type "/Game/BP_SaveGame Object Reference"))
  (bind _currentdialogueid (`self.CurrentDialogueID`))
  ; OnSave and OnLoad event dispatchers from GameMode called so it can save the data of where the players are in the dialogue hierarchy
  (`BlueprintMapLibrary.Map_Add` (`/Game/BP_SaveGame.NPCDialogueData` SaveGame) (`self.NPC_ID`) (make `/Game/S_NPCDialogueSaveData` _currentdialogueid))
  (`KismetSystemLibrary.PrintString` (`KismetStringLibrary.Conv_NameToString` _currentdialogueid)))

(event `OnLoad_Event`
  (params (SaveGame :type "/Game/BP_SaveGame Object Reference"))
  (bind (_value _returnvalue) (`BlueprintMapLibrary.Map_Find` (`/Game/BP_SaveGame.NPCDialogueData` SaveGame) (`self.NPC_ID`)))
  ; OnSave and OnLoad event dispatchers from GameMode called so it can save the data of where the players are in the dialogue hierarchy
  (if _returnvalue
    (bind _output_get (set `self.CurrentDialogueID` (`.CurrentDialogueID_2_60062D204F99946EDC0D95BBA9EDD589` (break `/Game/S_NPCDialogueSaveData` _value))))
    (bind _returnvalue_2 (`|GetDataTableRow` (`self.DialogueTable`) _output_get)
      (:`then`
        (bind _output_get_2 (set `self.CurrentDialogueData` _returnvalue_2))
        (set `self.currentDialogueTable` (break `/Game/Dialogue/S_DialogueStruct` _output_get_2))))))

(fn `AdvanceDialogue`
  (bind (_currentnodedata_nodeid _currentnodedata_speakername _currentnodedata_dialoguetext _currentnodedata_nextnodeid _currentnodedata_choicesp1) (break `/Game/Dialogue/S_DialogueNode` (`self.CurrentNodeData`)))
  (bind (_currentnodedata_nodeid_2 _currentnodedata_speakername_2 _currentnodedata_dialoguetext_2 _currentnodedata_nextnodeid_2 _currentnodedata_choicesp1_2 _currentnodedata_choicesp2) (break `/Game/Dialogue/S_DialogueNode` (`self.CurrentNodeData`)))
  (bind (_currentnodedata_nodeid_3 _currentnodedata_speakername_3 _currentnodedata_dialoguetext_3 _currentnodedata_nextnodeid_3 _currentnodedata_choicesp1_3 _currentnodedata_choicesp2_2) (break `/Game/Dialogue/S_DialogueNode` (`self.CurrentNodeData`)))
  ; Get the new current node data from current dialogue table and current node ID
  (if (`self.bDialogueActive`)
    (bind _returnvalue (`|GetDataTableRow` (`self.currentDialogueTable`) (`self.CurrentNodeID`))
      (:`then`
        (set `self.CurrentNodeData` _returnvalue)
        ; For each player : update their dialogues widget with the new data (name of the person talking, text, if there is choices or not)
        (for _array_element (`GameStateBase.PlayerArray` (`GameplayStatics.GetGameState`))
          (bind _asbp_third_person_player_controller (cast `/Game/ThirdPerson/Blueprints/BP_ThirdPersonPlayerController` (`PlayerState.GetPlayerController` _array_element)))
          (if (== _asbp_third_person_player_controller (`GameplayStatics.GetPlayerController` 0))
            (`/Game/ThirdPerson/Blueprints/BP_ThirdPersonPlayerController.Client_UpdateDialogueFromNPC` _asbp_third_person_player_controller _currentnodedata_speakername _currentnodedata_dialoguetext _currentnodedata_choicesp1)
            (else
              (`/Game/ThirdPerson/Blueprints/BP_ThirdPersonPlayerController.Client_UpdateDialogueFromNPC` _asbp_third_person_player_controller _currentnodedata_speakername_2 _currentnodedata_dialoguetext_2 _currentnodedata_choicesp2))))
        ; If array choices are not empty, wait for the choices of the players for the dialogue to continue, else currentNodeID is updated or dialogue is ended if this is the end of the dialogue (nextNodeID is empty)
        (if (and (`KismetArrayLibrary.Array_IsNotEmpty` _currentnodedata_choicesp1_3) (`KismetArrayLibrary.Array_IsNotEmpty` _currentnodedata_choicesp2_2))
          (`KismetSystemLibrary.PrintString` "There is choices")
          (elif (!= _currentnodedata_nextnodeid_3 "None")
            (set `self.CurrentNodeID` _currentnodedata_nextnodeid_3)
            (else
              (`KismetSystemLibrary.PrintString` "One of the two array choices isnt filled")
              (`self.EndDialogue`))))))))

(fn `CheckItemTag`
  (bind (_currentdialoguedata_nodeid _currentdialoguedata_nextdialoguename _currentdialoguedata_possessitemtag) (break `/Game/Dialogue/S_DialogueStruct` (`self.CurrentDialogueData`)))
  ; Verify if current dialogue Data Tag list is empty
  (if (`BlueprintMapLibrary.Map_IsNotEmpty` _currentdialoguedata_possessitemtag)
    ; If not empty, check if it's tag is contained is the gameTagContainer list in GameInstance
    (bind _asbp_game_instance (cast `/Game/Core/BP_GameInstance` (`GameplayStatics.GetGameInstance`)))
    (bind (_keypin _valuepin) (`|MapForEach` _currentdialoguedata_possessitemtag :!label _label)
      (:`then`
        (bind _hastag (`/Game/BP_StateTags.HasGameTag` (`/Game/Core/BP_GameInstance.stateTags` _asbp_game_instance) _keypin))
        (if _hastag
          ; If it is in, get the new dialogue data from the row names associated with the tag and set the new values
          (bind _returnvalue (`|GetDataTableRow` (`self.DialogueTable`) _valuepin)
            (:`then`
              (bind _output_get (set `self.CurrentDialogueData` _returnvalue))
              (set `self.currentDialogueTable` (break `/Game/Dialogue/S_DialogueStruct` _output_get))
              (set `self.CurrentDialogueID` _valuepin)
              (goto _label :!via `BreakPin`))))))))

(fn `ChoiceAdvanceDialogue`
  (params (`Choice ID` :type Integer) (PlayerController :type "/Game/ThirdPerson/Blueprints/BP_ThirdPersonPlayerController Object Reference"))
  (locals (IDChoice :type Integer))
  (bind (_currentdialoguedata_nodeid _currentdialoguedata_nextdialoguename) (break `/Game/Dialogue/S_DialogueStruct` (`self.CurrentDialogueData`)))
  (bind (_currentnodedata_nodeid _currentnodedata_speakername _currentnodedata_dialoguetext _currentnodedata_nextnodeid _currentnodedata_choicesp1 _currentnodedata_choicesp2 _currentnodedata_nextdialogue) (break `/Game/Dialogue/S_DialogueNode` (`self.CurrentNodeData`)))
  ; Update "ChoiceIDP1" or "ChoiceIDP2" int variable if it's P1 player or P2 player calling the function
  (if (`self.bDialogueActive`)
    (if (== PlayerController (`GameplayStatics.GetPlayerController` 0))
      (set `self.Choice ID P1` `Choice ID`)
      (else
        (set `self.Choice ID P2` `Choice ID`)))
    ; If both players have selected a choice (ChoiceIDP1/2 != -1) then TotalPointChoice is calculated and can get the next dialogue
    (if (and (!= (`self.Choice ID P1`) -1) (!= (`self.Choice ID P2`) -1))
      (set `self.TotalPointChoice` (+ (`self.Choice ID P1`) (`self.Choice ID P2`)))
      ; Get the next DialogueID (update the NextDialogueID? variable so we can check later that a choice has been selected), update CurrentNodeID and advance the dialogue if there is a next node
      (bind _choiceid (`self.GetNextDialogueID`))
      (set `self.NextDialogueID?` (`|GetArrayItem` _currentdialoguedata_nextdialoguename _choiceid))
      (if (`KismetArrayLibrary.Array_IsNotEmpty` _currentnodedata_nextdialogue)
        (set `self.CurrentNodeID` (`|GetArrayItem` _currentnodedata_nextdialogue _choiceid))
        (`self.ResetDialogueChoiceValue`)
        (`self.AdvanceDialogue`)
        (else
          (`self.EndDialogue`))))))

(fn `EndDialogue`
  ; Reset values to default or null and call each client (players) to end the dialogue
  (set `self.bDialogueActive` false)
  (set `self.CurrentNodeID` "Start")
  (set `self.CurrentNodeData` (struct))
  (`self.SetNextDialogueData`)
  (`self.ResetDialogueChoiceValue`)
  (for _array_element (`GameStateBase.PlayerArray` (`GameplayStatics.GetGameState`))
    (bind _asbp_third_person_player_controller (cast `/Game/ThirdPerson/Blueprints/BP_ThirdPersonPlayerController` (`PlayerState.GetPlayerController` _array_element)))
    (`/Game/ThirdPerson/Blueprints/BP_ThirdPersonPlayerController.Client_EndDialogue` _asbp_third_person_player_controller)))

(fn `GetNextDialogueID`
  (returns (ChoiceID :type Integer))
  ; Return the correct ChoiceID value depending on choices of player 1 and 2 (Positif, Negatif, Orange, Violet) ID Value = 0 =positif / 1 = orange / 2 = Violet / 3 = Rouge
  (if (>= (`self.TotalPointChoice`) 2)
    (`KismetSystemLibrary.PrintString` "Choix positif")
    (return 0)
    (elif (<= (`self.TotalPointChoice`) -2)
      (`KismetSystemLibrary.PrintString` "Choix negatif")
      (return 3)
      (elif (== (`self.Choice ID P1`) (`self.Choice ID P2`))
        (`KismetSystemLibrary.PrintString` "Orange")
        (return 1)
        (else
          (`KismetSystemLibrary.PrintString` "Violet")
          (return 2))))))

(fn `InitDialogue`
  (returns (InitDialogueData :type "/Game/Dialogue/S_DialogueNode Structure"))
  (bind (_currentnodedata_nodeid _currentnodedata_speakername _currentnodedata_dialoguetext _currentnodedata_nextnodeid) (break `/Game/Dialogue/S_DialogueNode` (`self.CurrentNodeData`)))
  ; Get the CurrentNodeData from current dialogue table and nodeID, if there is not a next nodeID, call endDialogue, else return data for dialogue to be initialize
  (bind _returnvalue (`|GetDataTableRow` (`self.currentDialogueTable`) (`self.CurrentNodeID`))
    (:`then`
      (bind _output_get (set `self.CurrentNodeData` _returnvalue))
      (if (!= _currentnodedata_nextnodeid "None")
        (set `self.CurrentNodeID` _currentnodedata_nextnodeid)
        (set `self.bDialogueActive` true)
        (return _output_get)
        (else
          (`self.EndDialogue`))))))

(fn `OnRep_Opened?`)

(fn `ResetDialogueChoiceValue`
  ; Reset Dialogue Value if there was a choice
  (set `self.Choice ID P1` -1)
  (set `self.Choice ID P2` -1)
  (set `self.TotalPointChoice` 0)
  (set `self.IDChoice` -1))

(fn `SetNextDialogueData`
  (bind (_currentdialoguedata_nodeid _currentdialoguedata_nextdialoguename) (break `/Game/Dialogue/S_DialogueStruct` (`self.CurrentDialogueData`)))
  (bind _nextdialogueid_ (`self.NextDialogueID?`))
  (bind _output (`|GetArrayItem` _currentdialoguedata_nextdialoguename))
  ; Is true if we had a choices earlier in the dialogue
  (if (== (`self.NextDialogueID?`) "None")
    ; Get Data to set up the next dialogue with the default next dialogue from the dialogueData
    (bind _returnvalue (`|GetDataTableRow` (`self.DialogueTable`) _output)
      (:`then`
        (set `self.CurrentDialogueID` _output)
        (bind _output_get (set `self.CurrentDialogueData` _returnvalue))
        (set `self.currentDialogueTable` (break `/Game/Dialogue/S_DialogueStruct` _output_get))))
    (else
      ; Get data to set up the next dialogue with the row name from the choices
      (bind _returnvalue_2 (`|GetDataTableRow` (`self.DialogueTable`) _nextdialogueid_)
        (:`then`
          (set `self.CurrentDialogueID` _nextdialogueid_)
          (bind _output_get_2 (set `self.CurrentDialogueData` _returnvalue_2))
          (set `self.currentDialogueTable` (break `/Game/Dialogue/S_DialogueStruct` _output_get_2))
          (set `self.NextDialogueID?` "None"))))))