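; BP_StateTags holds the game's state gameplay tags, keeping GameInstance tag logic in a separate Blueprint for clarity.
; It exposes functions to query a tag, add a tag and return the whole GameTagsContainer.
; Queries use exact matching, and adding first checks for duplicates, printing a debug string for either outcome.
; No function here removes tags.
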(fn `AddGameTag`
  (params (GameTag :type "GameplayTag Structure"))
  (bind _gametagscontainer (`self.gameTagsContainer`))
  ; Function that add a GameTag to the GameTagContainer if it's not in it already
  (if (`BlueprintGameplayTagLibrary.HasTag` _gametagscontainer GameTag true)
    (`KismetSystemLibrary.PrintString` null "Tag already in")
    (else
      (`KismetSystemLibrary.PrintString` null "Add tag")
      (`BlueprintGameplayTagLibrary.AddGameplayTag` _gametagscontainer GameTag))))

(fn `GetGameTagsContainer`
  (returns (gameTagsContainer :type "GameplayTagContainer Structure"))
  ; Function that return the gametagContainer of GameInstance
  (return (`self.gameTagsContainer`)))

(fn `HasGameTag`
  (params (GameTag :type "GameplayTag Structure"))
  (returns (HasTag :type Boolean))
  ; Function that verify if gametag input is contained in the gametag container of gameinstance (put every GameInstance function related to gameTag inside BP StateTags instead for clarity of GameInstance)
  (return (`BlueprintGameplayTagLibrary.HasTag` (`self.gameTagsContainer`) GameTag true)))